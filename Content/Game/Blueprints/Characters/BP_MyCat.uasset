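; BP_MyCat is a Paper2D cat character that animates its replicated sprite according to movement and jumping.
; Tick advances a jump state through start, process and finish phases, using short delays and the movement component's falling check.
; UpdateAnimation feeds that state and IsMoving into AnimationStateMachine, which selects the flipbook.
; SoundStateMachine is an empty stub, and a disconnected animation branch holds unused hitting and interacting checks.
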(event `self.ReceiveBeginPlay`
  (`ActorComponent.SetIsReplicated` (`self.Sprite`) true))

(event `UpdateAnimation`
  (bind _result_flipbook (`self.AnimationStateMachine` (`self.IsMoving`) (`self.JumpingState`) (`self.IsHitting`) (`NavMovementComponent.IsFalling` (`self.CharacterMovement`))))
  (`PaperFlipbookComponent.SetFlipbook` (`self.Sprite`) _result_flipbook))

(event `self.ReceiveTick`
  (params (DeltaSeconds :type "Float (single-precision)"))
  (`self.UpdateJumpingState`)
  (`self.SoundStateMachine`))

(event `UpdateJumpingState`
  (switch `/Game/Game/Blueprints/Data/JumpStates` (`self.JumpingState`)
    (:`NewEnumerator0`
      (if (`NavMovementComponent.IsFalling` (`self.CharacterMovement`))
        ;[1 1 1] падает не прыгает
        (set `self.JumpingState` "NewEnumerator2")
        (else
          ;[1 1 1] не прігает не падает
          (set `self.JumpingState` "NewEnumerator0"))))
    (:`NewEnumerator1`
      ;[1 1 1] Таймер не установлен
      (set `self.JumpingState` "NewEnumerator1")
      (`KismetSystemLibrary.Delay` 0.2)
      (set `self.JumpingState` "NewEnumerator2")
      (`self.UpdateAnimation`))
    (:`NewEnumerator2`
      (if (`NavMovementComponent.IsFalling` (`self.CharacterMovement`))
        ;[1 1 1] Еще не упал
        (set `self.JumpingState` "NewEnumerator2")
        (else
          (set `self.JumpingState` "NewEnumerator3")
          (`KismetSystemLibrary.Delay` 0.15)
          (set `self.JumpingState` "NewEnumerator0")
          (`self.UpdateAnimation`))))))

(fn `AnimationStateMachine`
  (params (IsMoving :type Boolean) (JumpingState :type "/Game/Game/Blueprints/Data/JumpStates Enum" :default "NewEnumerator0") (IsHitting :type Boolean) (IsFalling :type Boolean))
  (returns (`Result Flipbook` :type "PaperFlipbook Object Reference"))
  (locals (States :type "/Game/Game/Blueprints/Data/States Enum") (IsFallingLocal :type Boolean))
  (set `local.IsFallingLocal` IsFalling)
  (switch `/Game/Game/Blueprints/Data/JumpStates` JumpingState
    (:`NewEnumerator0`
      (if (`self.IsMoving`)
        (set `self.State` "NewEnumerator1")
        (else
          (set `self.State` "NewEnumerator0"))))
    (:`NewEnumerator1`
      (set `self.State` "NewEnumerator3"))
    (:`NewEnumerator2`
      (set `self.State` "NewEnumerator4"))
    (:`NewEnumerator3`
      (set `self.State` "NewEnumerator5")))
  (return (select `/Game/Game/Blueprints/Data/States` (`self.State`) :`NewEnumerator0` (`self.IdleFlipbook`) :`NewEnumerator1` (`self.WalkingFlipbook`) :`NewEnumerator3` (`self.JumpStartFlipbook`) :`NewEnumerator4` (`self.JumpProcessFlipbook`) :`NewEnumerator5` (`self.JumpFinishFlipBook`))))

(fn `SoundStateMachine`)

(fn `UserConstructionScript`)