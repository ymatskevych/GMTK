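; BP_AliveCat is the living cat Paper2D character, paired with a ghost counterpart via AnotherCat.
; Tick advances a jump state machine with timed start and landing phases, while UpdateAnimation maps movement and jump state to flipbooks.
; Damage reduces HP; at zero or below, input is disabled, both cats show death flipbooks and the level restarts.
; Capsule overlap with a BP_AliveCat triggers CallJoiningHappened.
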(event `self.ReceiveBeginPlay`
  (`ActorComponent.SetIsReplicated` (`self.Sprite`) true))

(event `UpdateAnimation`
  (bind _result_flipbook (`self.AnimationStateMachine` (`self.IsMoving`) (`self.JumpingState`) (`self.IsHitting`) (`NavMovementComponent.IsFalling` (`self.CharacterMovement`))))
  (`PaperFlipbookComponent.SetFlipbook` (`self.Sprite`) _result_flipbook))

(event `self.ReceiveTick`
  (params (DeltaSeconds :type "Float (single-precision)"))
  (`self.UpdateJumpingState`))

(event `UpdateJumpingState`
  (switch `/Game/Game/Blueprints/Data/JumpStates` (`self.JumpingState`)
    (:`NewEnumerator0`
      (if (`NavMovementComponent.IsFalling` (`self.CharacterMovement`))
        ;[1 1 1] падает не прыгает
        (set `self.JumpingState` "NewEnumerator2")
        (else
          ;[1 1 1] не прігает не падает
          (set `self.JumpingState` "NewEnumerator0"))))
    (:`NewEnumerator1`
      ;[1 1 1] Таймер не установлен
      (set `self.JumpingState` "NewEnumerator1")
      (`KismetSystemLibrary.Delay` 0.2)
      (set `self.JumpingState` "NewEnumerator2")
      (`self.UpdateAnimation`))
    (:`NewEnumerator2`
      (if (`NavMovementComponent.IsFalling` (`self.CharacterMovement`))
        ;[1 1 1] Еще не упал
        (set `self.JumpingState` "NewEnumerator2")
        (else
          (set `self.JumpingState` "NewEnumerator3")
          (`KismetSystemLibrary.Delay` 0.15)
          (set `self.JumpingState` "NewEnumerator0")
          (`self.UpdateAnimation`))))))

(event `self.ReceiveAnyDamage`
  (params (Damage :type "Float (single-precision)") (DamageType :type "DamageType Object Reference") (InstigatedBy :type "Controller Object Reference") (DamageCauser :type "Actor Object Reference"))
  (set `self.HP` (- (`self.HP`) Damage))
  (bind _isdead (`self.CheckDeath`))
  (if _isdead
    (`self.Die `)))

(event `Die`
  (bind _returnvalue (`GameplayStatics.GetPlayerController` 0))
  (`KismetSystemLibrary.PrintString` "Die")
  (`self.DisableInput` _returnvalue _returnvalue)
  (`KismetSystemLibrary.Delay` 0.2)
  (`PaperFlipbookComponent.SetFlipbook` (`self.Sprite`) "/Game/Game/Resources/Textures/FP_AliveDeath.FP_AliveDeath")
  (`PaperFlipbookComponent.SetFlipbook` (`PaperCharacter.Sprite` (`self.AnotherCat`)) "/Game/Game/Resources/Textures/FB_GhostDeath.FB_GhostDeath")
  (`KismetSystemLibrary.Delay` 0.8)
  (`KismetSystemLibrary.ExecuteConsoleCommand` "RestartLevel" null))

(event `self.CapsuleComponent.OnComponentBeginOverlap`
  (params (OverlappedComponent :type "PrimitiveComponent Object Reference") (OtherActor :type "Actor Object Reference") (OtherComp :type "PrimitiveComponent Object Reference") (OtherBodyIndex :type Integer) (bFromSweep :type Boolean) (SweepResult :type "HitResult Structure (by ref)"))
  (cast `/Game/Game/Blueprints/Characters/BP_AliveCat` OtherActor)
  (`self.JoiningHappened`))

(fn `AnimationStateMachine`
  (params (IsMoving :type Boolean) (JumpingState :type "/Game/Game/Blueprints/Data/JumpStates Enum" :default "NewEnumerator0") (IsHitting :type Boolean) (IsFalling :type Boolean))
  (returns (`Result Flipbook` :type "PaperFlipbook Object Reference"))
  (locals (States :type "/Game/Game/Blueprints/Data/States Enum") (IsFallingLocal :type Boolean))
  (set `local.IsFallingLocal` IsFalling)
  (switch `/Game/Game/Blueprints/Data/JumpStates` JumpingState
    (:`NewEnumerator0`
      (if (`self.IsMoving`)
        (set `self.State` "NewEnumerator1")
        (else
          (set `self.State` "NewEnumerator0"))))
    (:`NewEnumerator1`
      (set `self.State` "NewEnumerator3"))
    (:`NewEnumerator2`
      (set `self.State` "NewEnumerator4"))
    (:`NewEnumerator3`
      (set `self.State` "NewEnumerator5")))
  (return (select `/Game/Game/Blueprints/Data/States` (`self.State`) :`NewEnumerator0` (`self.IdleFlipbook`) :`NewEnumerator1` (`self.WalkingFlipbook`) :`NewEnumerator3` (`self.JumpStartFlipbook`) :`NewEnumerator4` (`self.JumpProcessFlipbook`) :`NewEnumerator5` (`self.JumpFinishFlipBook`))))

(fn `CheckDeath`
  (returns (IsDead :type Boolean))
  (return (<= (`self.HP`) 0.0)))

(fn `SoundStateMachine`)

(fn `UserConstructionScript`)