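; Game mode, apparently for an opening text-crawl level, that moves on to the first level after a fixed delay.
; A BeginPlay timer opens FLevel1, restores game-only input and starts music through BP_GameInstance.
; It also creates a collapsed pause widget whose buttons return to MainMenu or resume play, restoring input and notifying the game instance.
; Nothing in this graph shows the pause menu.
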(event `CreatePauseMenu`
  (bind _returnvalue (`|CreateWidget` "/Game/Game/Blueprints/UI/W_Pause.W_Pause_C"))
  (bind _output_get (set `self.PauseWidget` _returnvalue))
  (`UserWidget.AddToViewport` _output_get 0)
  (`Widget.SetVisibility` _output_get "Collapsed")
  (add `Button.OnClicked` (`/Game/Game/Blueprints/UI/W_Pause.Button_MainMenu` _output_get) (delegate `OnMainMenu`))
  (add `Button.OnClicked` (`/Game/Game/Blueprints/UI/W_Pause.Button_Continue` _output_get) (delegate `OnContinueGame`)))

(event `OnContinueGame`
  (bind _returnvalue (`GameplayStatics.GetPlayerController` 0))
  (`self.GameContinue`)
  (set `PlayerController.bShowMouseCursor` false _returnvalue)
  (`Widget.SetVisibility` (`self.PauseWidget`) "Collapsed")
  (`WidgetBlueprintLibrary.SetInputMode_GameOnly` _returnvalue)
  (`GameplayStatics.SetGamePaused` false)
  (bind _asbp_game_instance (cast `/Game/Game/Blueprints/GameModes/BP_GameInstance` (`GameplayStatics.GetGameInstance`)))
  (`/Game/Game/Blueprints/GameModes/BP_GameInstance.Unpause` _asbp_game_instance))

(event `OnMainMenu`
  (`GameplayStatics.OpenLevel` "MainMenu")
  (`Widget.RemoveFromParent` (`self.PauseWidget`)))

(event `self.ReceiveBeginPlay`
  (`KismetSystemLibrary.K2_SetTimerDelegate` (delegate `Level1Opening`) 30.0)
  (`self.CreatePauseMenu`))

(event `Level1Opening`
  (`GameplayStatics.OpenLevel` "FLevel1")
  (`WidgetBlueprintLibrary.SetInputMode_GameOnly` (`GameplayStatics.GetPlayerController` 0))
  (bind _asbp_game_instance (cast `/Game/Game/Blueprints/GameModes/BP_GameInstance` (`GameplayStatics.GetGameInstance`)))
  (`/Game/Game/Blueprints/GameModes/BP_GameInstance.StartPlaySound` _asbp_game_instance "/Game/Game/Resources/Sounds/Komiku_-_03_-_Mushrooms_Cue.Komiku_-_03_-_Mushrooms_Cue"))

(fn `UserConstructionScript`)