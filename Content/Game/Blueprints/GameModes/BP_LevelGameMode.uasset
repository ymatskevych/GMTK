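; Level game mode that builds and manages the in-level pause menu widget.
; On BeginPlay it creates W_Pause, adds it to the viewport collapsed and binds its Continue and Main Menu buttons.
; Continue calls CallGameContinue, hides the cursor and menu, restores game-only input and unpauses; Main Menu opens the MainMenu level.
; Nothing in this graph shows the menu or pauses the game.
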(event `CreatePauseMenu`
  (bind _returnvalue (`|CreateWidget` "/Game/Game/Blueprints/UI/W_Pause.W_Pause_C"))
  (bind _output_get (set `self.PauseWidget` _returnvalue))
  (`UserWidget.AddToViewport` _output_get 0)
  (`Widget.SetVisibility` _output_get "Collapsed")
  (add `Button.OnClicked` (`/Game/Game/Blueprints/UI/W_Pause.Button_MainMenu` _output_get) (delegate `OnMainMenu`))
  (add `Button.OnClicked` (`/Game/Game/Blueprints/UI/W_Pause.Button_Continue` _output_get) (delegate `OnContinueGame`)))

(event `OnContinueGame`
  (bind _returnvalue (`GameplayStatics.GetPlayerController` 0))
  (`self.GameContinue`)
  (set `PlayerController.bShowMouseCursor` false _returnvalue)
  (`Widget.SetVisibility` (`self.PauseWidget`) "Collapsed")
  (`WidgetBlueprintLibrary.SetInputMode_GameOnly` _returnvalue)
  (`GameplayStatics.SetGamePaused` false))

(event `OnMainMenu`
  (`GameplayStatics.OpenLevel` "MainMenu")
  (`Widget.RemoveFromParent` (`self.PauseWidget`)))

(event `self.ReceiveBeginPlay`
  (`self.CreatePauseMenu`))

(fn `UserConstructionScript`)