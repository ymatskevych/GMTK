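; Main menu game mode that shows the menu widget and starts menu music when the level begins.
; On BeginPlay it creates W_MainMenu, binds its Play and Exit buttons, and switches to UI-only input with a visible cursor.
; Play opens the LevelCrowlText level, removes the menu, restores game input and changes the music through BP_GameInstance.
; Exit quits the game.
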(event `OnPlayButtonClicked`
  (`GameplayStatics.OpenLevel` "LevelCrowlText")
  (`Widget.RemoveFromParent` (`self.Main Menu Widjet`))
  (`WidgetBlueprintLibrary.SetInputMode_GameOnly` (`GameplayStatics.GetPlayerController` 0))
  (bind _asbp_game_instance (cast `/Game/Game/Blueprints/GameModes/BP_GameInstance` (`GameplayStatics.GetGameInstance`)))
  (`/Game/Game/Blueprints/GameModes/BP_GameInstance.StartPlaySound` _asbp_game_instance "/Game/Game/Resources/Sounds/BestVocalDuet_Cue.BestVocalDuet_Cue"))

(event `CreateMainMenu`
  (bind _returnvalue (`GameplayStatics.GetPlayerController` 0))
  (bind _returnvalue_2 (`|CreateWidget` "/Game/Game/Blueprints/UI/W_MainMenu.W_MainMenu_C"))
  (`UserWidget.AddToViewport` _returnvalue_2 0)
  (set `self.Main Menu Widjet` _returnvalue_2)
  (`|ExecutionSequence`
    (:`then_0`
      (add `Button.OnClicked` (`/Game/Game/Blueprints/UI/W_MainMenu.Button_Play` (`self.Main Menu Widjet`)) (delegate `OnPlayButtonClicked`)))
    (:`then_1`
      (add `Button.OnClicked` (`/Game/Game/Blueprints/UI/W_MainMenu.Button_Exit` (`self.Main Menu Widjet`)) (delegate `OnExitButtonClicked`)))
    (:`then_2`
      (set `PlayerController.bShowMouseCursor` true _returnvalue)
      (`WidgetBlueprintLibrary.SetInputMode_UIOnlyEx` _returnvalue (`self.Main Menu Widjet`)))))

(event `self.ReceiveBeginPlay`
  (`self.CreateMainMenu`)
  (bind _asbp_game_instance (cast `/Game/Game/Blueprints/GameModes/BP_GameInstance` (`GameplayStatics.GetGameInstance`)))
  (`/Game/Game/Blueprints/GameModes/BP_GameInstance.StartPlaySound` _asbp_game_instance "/Game/Game/Resources/Sounds/Komiku_-_03_-_Mushrooms_Cue.Komiku_-_03_-_Mushrooms_Cue"))

(event `OnExitButtonClicked`
  (`KismetSystemLibrary.QuitGame` null "Quit"))

(fn `UserConstructionScript`)