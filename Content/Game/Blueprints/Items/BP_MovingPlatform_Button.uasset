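; A moving platform variant that begins endlessly shuttling back and forth once its floor button is pressed.
; On BeginPlay it binds to the button in its child actor component and scales two timelines' play rates by a speed modifier.
; After an initial delay, a looping delay chain alternates forward and return moves, with waits derived from that modifier plus a direction-switch pause.
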(event `self.ReceiveBeginPlay`
  (bind _speedmodifier (`self.SpeedModifier`))
  (`parent.ReceiveBeginPlay`)
  (bind _asbp_floor_button (cast `/Game/Game/Blueprints/Items/BP_FloorButton` (`ChildActorComponent.ChildActor` (`self.ButtonActor`))))
  (add `/Game/Game/Blueprints/Items/BP_FloorButton.OnPressed` _asbp_floor_button (delegate `OnPressed`))
  (`TimelineComponent.SetPlayRate` (`self.Timeline_0`) _speedmodifier)
  (`TimelineComponent.SetPlayRate` (`self.Timeline_1`) _speedmodifier))

(event `OnPressed`
  (bind _returnvalue (/ 5.0 (`self.SpeedModifier`)))
  (`KismetSystemLibrary.Delay` (`self.InitialDelay`))
  (`self.MovePlatform` :!label _label)
  (`KismetSystemLibrary.Delay` (+ (`self.SwitchDirectionDelay`) _returnvalue))
  (`self.MovePlatformBack`)
  (`KismetSystemLibrary.Delay` (+ (`self.SwitchDirectionDelay`) _returnvalue))
  (goto _label))

(fn `UserConstructionScript`
  (`parent.UserConstructionScript`))