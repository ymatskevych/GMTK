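; Moving platform variant driven by a floor button: it moves after the button is pressed and stops when released.
; On BeginPlay it binds to the BP_FloorButton child actor's press and release events, passes it the cat type and scales the timeline's play rate.
; Pressing waits an initial delay before moving, while releasing stops movement and sets a paused flag.
; Tick stops the timeline whenever it plays while paused.
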(event `self.ReceiveBeginPlay`
  (`parent.ReceiveBeginPlay`)
  (bind _asbp_floor_button (cast `/Game/Game/Blueprints/Items/BP_FloorButton` (`ChildActorComponent.ChildActor` (`self.ButtonActor`))))
  (add `/Game/Game/Blueprints/Items/BP_FloorButton.OnPressed` _asbp_floor_button (delegate `OnPressed`))
  (add `/Game/Game/Blueprints/Items/BP_FloorButton.OnUnpressed` _asbp_floor_button (delegate `OnUnpressedButton`))
  (`TimelineComponent.SetPlayRate` (`self.Timeline_0`) (`self.SpeedModifier`))
  (bind _asbp_floor_button_2 (cast `/Game/Game/Blueprints/Items/BP_FloorButton` (`ChildActorComponent.ChildActor` (`self.ButtonActor`)))
    (:`then`
      (set `/Game/Game/Blueprints/Items/BP_FloorButton.ButtonCatType` (`self.ButtonCatType`) _asbp_floor_button_2))
    (:`CastFailed`
      (`KismetSystemLibrary.PrintString` "Cast to bp_flootbutton failed (BP_MovingPlatform_Button)"))))

(event `OnPressed`
  (`KismetSystemLibrary.Delay` (`self.InitialDelay`))
  (`self.MovePlatform`)
  (set `self.IsPaused` false))

(event `OnUnpressedButton`
  (`self.StopMoving`)
  (set `self.IsPaused` true))

(event `self.ReceiveTick`
  (params (DeltaSeconds :type "Float (single-precision)"))
  (bind _timeline_0 (`self.Timeline_0`))
  (if (`self.IsPaused`)
    (if (`TimelineComponent.IsPlaying` _timeline_0)
      (`TimelineComponent.Stop` _timeline_0))))

(fn `UserConstructionScript`
  (`parent.UserConstructionScript`))