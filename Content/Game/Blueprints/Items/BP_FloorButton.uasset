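; Floor button that reacts to the player cat stepping on it, filtered by whether it accepts only alive cats, only dead cats or all.
; Trigger overlap latches Pressed, then calls OnPressed and turns the sprite green if the cat's type matches.
; Any Character leaving clears the state, calls OnUnpressed and turns it red.
; IsPressed exposes the flag, which is set even when the type does not match.
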(event `self.Trigger.OnComponentBeginOverlap`
  (params (OverlappedComponent :type "PrimitiveComponent Object Reference") (OtherActor :type "Actor Object Reference") (OtherComp :type "PrimitiveComponent Object Reference") (OtherBodyIndex :type Integer) (bFromSweep :type Boolean) (SweepResult :type "HitResult Structure (by ref)"))
  (bind _buttoncattype (`self.ButtonCatType`))
  (bind _asbp_my_cat (cast `/Game/Game/Blueprints/Characters/BP_MyCat` OtherActor)
    (:`then`
      (if (not (`self.Pressed`))
        (set `self.Pressed` true)
        (switch `/Game/Game/Blueprints/Enums/EPlatformState` _buttoncattype
          (:`NewEnumerator1`
            (bind _returnvalue (`|EnumEquality` (`/Game/Game/Blueprints/Characters/BP_MyCat.CatType` _asbp_my_cat) "NewEnumerator0"))
            (if _returnvalue :!label _label
              (if (and _returnvalue (`|EnumEquality` _buttoncattype "NewEnumerator1"))
                (`self.OnPressed` :!label _label_2)
                (`PaperSpriteComponent.SetSpriteColor` (`self.PaperSprite`) (struct :`G` 1.0 :`B` 0.122778 :`A` 1.0)))
              (elif (`|EnumEquality` _buttoncattype "NewEnumerator2")
                (goto _label_2))))
          (:`NewEnumerator2`
            (goto _label))
          (:`NewEnumerator3`
            (goto _label_2)))))
    (:`CastFailed`
      (`KismetSystemLibrary.PrintString` "Cast to character failed!!"))))

(event `self.Trigger.OnComponentEndOverlap`
  (params (OverlappedComponent :type "PrimitiveComponent Object Reference") (OtherActor :type "Actor Object Reference") (OtherComp :type "PrimitiveComponent Object Reference") (OtherBodyIndex :type Integer))
  (cast `Character` OtherActor
    (:`then`
      (set `self.Pressed` false)
      (`self.OnUnpressed`)
      (`PaperSpriteComponent.SetSpriteColor` (`self.PaperSprite`) (struct :`R` 1.0 :`G` 0.0169 :`A` 1.0)))
    (:`CastFailed`
      (`KismetSystemLibrary.PrintString` "Cast to character failed!!"))))

(fn `IsPressed`
  (returns (Pressed :type Boolean))
  (return (`self.Pressed`)))

(fn `UserConstructionScript`)