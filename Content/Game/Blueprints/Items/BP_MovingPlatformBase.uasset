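; Base Blueprint for a moving platform that shuttles a Paper2D sprite back and forth along an editor-placed arrow.
; MovePlatform runs a timeline that lerps from the start location to an X/Z endpoint derived from arrow length and pitch, pausing before each direction flip.
; When a Character overlaps ReverseTrigger, a ZHack height flag picks forward or reverse playback so the platform heads upward instead of into them.
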(event `self.ReceiveBeginPlay`
  (`parent.ReceiveBeginPlay`)
  (set `self.StartPoint` (`SceneComponent.K2_GetComponentLocation` (`self.PaperSprite`))))

(event `MovePlatform`
  (bind _startpoint (`self.StartPoint`))
  (bind _movingvector (`self.MovingVector`))
  (bind (_relativerotation_roll _relativerotation_pitch) (`KismetMathLibrary.BreakRotator` (`SceneComponent.RelativeRotation` _movingvector)))
  (bind _arrowlength (`ArrowComponent.ArrowLength` _movingvector))
  (bind (_direction _newtrack_0) (`Timeline|Timeline_0` :!label _label)
    (:`Update`
      (bind _returnvalue (`KismetMathLibrary.VLerp` _startpoint (+ (`self.StartPoint`) (`KismetMathLibrary.MakeVector` (* _arrowlength (`KismetMathLibrary.DegCos` _relativerotation_pitch)) 0.0 (* _arrowlength (`KismetMathLibrary.DegSin` _relativerotation_pitch)))) _newtrack_0))
      (`SceneComponent.K2_SetWorldLocation` (`self.PaperSprite`) _returnvalue false false)
      (set `self.ZHack` (< (- (.z _startpoint) (.z _returnvalue)) 0.0)))
    (:`Finished`
      (`KismetSystemLibrary.Delay` 2.0)
      (switch `ETimelineDirection` _direction
        (:`Forward`
          (goto _label :!via `Reverse`))
        (:`Backward`
          (goto _label))))))

(event `self.ReverseTrigger.OnComponentBeginOverlap`
  (params (OverlappedComponent :type "PrimitiveComponent Object Reference") (OtherActor :type "Actor Object Reference") (OtherComp :type "PrimitiveComponent Object Reference") (OtherBodyIndex :type Integer) (bFromSweep :type Boolean) (SweepResult :type "HitResult Structure (by ref)"))
  (bind _timeline_0 (`self.Timeline_0`))
  ;[1 1 1] Reverse platform moving when it crashes into player
  (cast `Character` OtherActor)
  (`TimelineComponent.Stop` _timeline_0)
  (if (`self.ZHack`)
    (`TimelineComponent.Play` _timeline_0)
    (else
      (`TimelineComponent.Reverse` _timeline_0))))

(fn `UserConstructionScript`
  (`parent.UserConstructionScript`))