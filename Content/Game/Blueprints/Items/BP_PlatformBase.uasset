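; Base 2D platform whose box collision is solid for no one, only alive cats, only dead cats, or all, depending on its PlatformState.
; BeginPlay sets fixed collision for the none and all states.
; Sprite overlaps and an enlarged per-tick box trace (debug-drawn) re-evaluate collision from the detected BP_AliveCat's CatType.
; OnAction applies the same state rule through IsValidForAction before calling DoAction, an empty hook for child Blueprints.
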(event `self.ReceiveBeginPlay`
  (bind _box (`self.Box`))
  (switch `/Game/Game/Blueprints/Enums/EPlatformState` (`self.PlatformState`)
    (:`NewEnumerator0`
      (`PrimitiveComponent.SetCollisionEnabled` _box "NoCollision"))
    (:`NewEnumerator3`
      (`PrimitiveComponent.SetCollisionEnabled` _box "QueryAndPhysics"))))

(event `OnAction`
  (params (PlayerState :type "/Game/Game/Blueprints/Enums/EPLayerState Enum" :default "NewEnumerator0"))
  (if (`self.IsValidForAction` PlayerState)
    (`self.DoAction`)))

(event `self.PaperSprite.OnComponentBeginOverlap`
  (params (OverlappedComponent :type "PrimitiveComponent Object Reference") (OtherActor :type "Actor Object Reference") (OtherComp :type "PrimitiveComponent Object Reference") (OtherBodyIndex :type Integer) (bFromSweep :type Boolean) (SweepResult :type "HitResult Structure (by ref)"))
  (bind _platformstate (`self.PlatformState`))
  (bind _box (`self.Box`))
  (bind _asbp_alive_cat (cast `/Game/Game/Blueprints/Characters/BP_AliveCat` OtherActor))
  (switch `/Game/Game/Blueprints/Enums/EPlatformState` _platformstate
    (:`NewEnumerator0`
      (`PrimitiveComponent.SetCollisionEnabled` _box "NoCollision" :!label _label))
    (:`NewEnumerator1`
      (bind _returnvalue (`|EnumEquality` (`/Game/Game/Blueprints/Characters/BP_AliveCat.CatType` _asbp_alive_cat) "NewEnumerator0"))
      (if _returnvalue :!label _label_2
        (if (and _returnvalue (`|EnumEquality` _platformstate "NewEnumerator1"))
          _
          (else
            (goto _label)))
        (elif (`|EnumEquality` _platformstate "NewEnumerator2")
          _
          (else
            (goto _label))))
      (`PrimitiveComponent.SetCollisionEnabled` _box "QueryAndPhysics" :!label _label_3))
    (:`NewEnumerator2`
      (goto _label_2))
    (:`NewEnumerator3`
      (goto _label_3))))

(event `self.ReceiveTick`
  (params (DeltaSeconds :type "Float (single-precision)"))
  (bind _box (`self.Box`))
  (bind _box_2 (`self.Box`))
  (bind _platformstate (`self.PlatformState`))
  (bind _returnvalue (`SceneComponent.K2_GetComponentLocation` _box))
  (bind _outhit (`KismetSystemLibrary.BoxTraceSingleForObjects` :`Start` _returnvalue :`End` _returnvalue :`HalfSize` (`KismetMathLibrary.MakeVector` (.x (* (`BoxComponent.GetScaledBoxExtent` _box) 1.25)) (.y (* (`BoxComponent.GetScaledBoxExtent` _box) 1.25)) (* (.z (* (`BoxComponent.GetScaledBoxExtent` _box) 1.25)) 1.5)) :`ObjectTypes` (`self.ObjectArray`) :`DrawDebugType` "ForOneFrame"))
  (bind _asbp_alive_cat (cast `/Game/Game/Blueprints/Characters/BP_AliveCat` (`.HitActor` (`GameplayStatics.BreakHitResult` _outhit))))
  (switch `/Game/Game/Blueprints/Enums/EPlatformState` _platformstate
    (:`NewEnumerator0`
      (`PrimitiveComponent.SetCollisionEnabled` _box_2 "NoCollision" :!label _label_4))
    (:`NewEnumerator1`
      (bind _returnvalue_2 (`|EnumEquality` (`/Game/Game/Blueprints/Characters/BP_AliveCat.CatType` _asbp_alive_cat) "NewEnumerator0"))
      (if _returnvalue_2 :!label _label_5
        (if (and _returnvalue_2 (`|EnumEquality` _platformstate "NewEnumerator1"))
          _
          (else
            (goto _label_4)))
        (elif (`|EnumEquality` _platformstate "NewEnumerator2")
          _
          (else
            (goto _label_4))))
      (`PrimitiveComponent.SetCollisionEnabled` _box_2 "QueryAndPhysics" :!label _label_6))
    (:`NewEnumerator2`
      (goto _label_5))
    (:`NewEnumerator3`
      (goto _label_6))))

(fn `DoAction`
  ;[1 1 1] To be implemented in children
)

(fn `IsValidForAction`
  (params (PlayerState :type "/Game/Game/Blueprints/Enums/EPLayerState Enum" :default "NewEnumerator0"))
  (returns (Valid :type Boolean))
  (bind _platformstate (`self.PlatformState`))
  (if (`|EnumEquality` PlayerState "NewEnumerator0")
    (switch `/Game/Game/Blueprints/Enums/EPlatformState` _platformstate
      (:`NewEnumerator0`
        _)
      (:`NewEnumerator1`
        (return true))
      (:`NewEnumerator2`
        _)
      (:`NewEnumerator3`
        (return true)))
    (else
      (switch `/Game/Game/Blueprints/Enums/EPlatformState` _platformstate
        (:`NewEnumerator0`
          _)
        (:`NewEnumerator1`
          _)
        (:`NewEnumerator2`
          (return true))
        (:`NewEnumerator3`
          (return true)))))
  (return false))

(fn `UserConstructionScript`)