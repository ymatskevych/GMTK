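; Moving platform variant toggled between forward and backward travel by a child floor button that shows the current state by color.
; BeginPlay binds the button's press event and passes it the cat type.
; After an initial delay, each press starts the opposite move or redirects a running movement timeline, then updates the button color.
; Tick stops Timeline0 whenever it plays, leaving movement to the other timelines and move functions.
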(event `self.ReceiveBeginPlay`
  (`parent.ReceiveBeginPlay`)
  (bind _asbp_floor_button (cast `/Game/Game/Blueprints/Items/BP_FloorButton` (`ChildActorComponent.ChildActor` (`self.ButtonActor`))))
  (add `/Game/Game/Blueprints/Items/BP_FloorButton.OnPressed` _asbp_floor_button (delegate `OnPressed`))
  (`TimelineComponent.SetPlayRate` (`self.Timeline_0`) (`self.SpeedModifier`))
  (bind _asbp_floor_button_2 (cast `/Game/Game/Blueprints/Items/BP_FloorButton` (`ChildActorComponent.ChildActor` (`self.ButtonActor`)))
    (:`then`
      (set `/Game/Game/Blueprints/Items/BP_FloorButton.ButtonCatType` (`self.ButtonCatType`) _asbp_floor_button_2)
      (`TimelineComponent.SetPlayRate` (`self.Timeline_0`) 1.0))
    (:`CastFailed`
      (`KismetSystemLibrary.PrintString` "Cast to bp_flootbutton failed (BP_MovingPlatform_Button)"))))

(event `OnPressed`
  (bind _timeline_1 (`self.Timeline_1`))
  (bind _timeline_2 (`self.Timeline_2`))
  (bind _childactor (`ChildActorComponent.ChildActor` (`self.ButtonActor`)))
  (bind _childactor_2 (`ChildActorComponent.ChildActor` (`self.ButtonActor`)))
  (`KismetSystemLibrary.Delay` (`self.InitialDelay`))
  (if (`TimelineComponent.IsPlaying` _timeline_1)
    (`TimelineComponent.Stop` _timeline_1)
    (`TimelineComponent.Reverse` _timeline_1)
    (set `self.IsForward` false)
    (bind _asbp_floor_button_state (cast `/Game/Game/Blueprints/Items/BP_FloorButton_State` _childactor))
    (`/Game/Game/Blueprints/Items/BP_FloorButton_State.SetState1Color` _asbp_floor_button_state)
    (elif (`TimelineComponent.IsPlaying` _timeline_2)
      (`TimelineComponent.Stop` _timeline_2)
      (`TimelineComponent.Play` _timeline_2)
      (set `self.IsForward` true)
      (bind _asbp_floor_button_state_2 (cast `/Game/Game/Blueprints/Items/BP_FloorButton_State` _childactor))
      (`/Game/Game/Blueprints/Items/BP_FloorButton_State.SetState2Color` _asbp_floor_button_state_2)
      (elif (`self.IsForward`)
        (`self.MoveBackward`)
        (set `self.IsForward` false)
        (bind _asbp_floor_button_state_3 (cast `/Game/Game/Blueprints/Items/BP_FloorButton_State` _childactor_2))
        (`/Game/Game/Blueprints/Items/BP_FloorButton_State.SetState1Color` _asbp_floor_button_state_3)
        (else
          (`self.MoveForward`)
          (set `self.IsForward` true)
          (bind _asbp_floor_button_state_4 (cast `/Game/Game/Blueprints/Items/BP_FloorButton_State` _childactor_2))
          (`/Game/Game/Blueprints/Items/BP_FloorButton_State.SetState2Color` _asbp_floor_button_state_4))))))

(event `self.ReceiveTick`
  (params (DeltaSeconds :type "Float (single-precision)"))
  (bind _timeline_0 (`self.Timeline_0`))
  (if (`TimelineComponent.IsPlaying` _timeline_0)
    (`TimelineComponent.Stop` _timeline_0)))

(fn `UserConstructionScript`
  (`parent.UserConstructionScript`))