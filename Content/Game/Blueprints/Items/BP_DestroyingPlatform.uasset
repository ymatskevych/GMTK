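; BP_DestroyingPlatform is a sprite platform that temporarily vanishes after the BP_MyCat character touches it.
; An overlap on DestroyTrigger starts a TimeToDestroy delay for any actor, with the cat cast checked only afterwards.
; For the cat, it hides the PaperSprite and disables its collision and the Box's.
; After TimeToRespawn, it restores visibility and collision, so the actor is never actually destroyed.
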(event `self.DestroyTrigger.OnComponentBeginOverlap`
  (params (OverlappedComponent :type "PrimitiveComponent Object Reference") (OtherActor :type "Actor Object Reference") (OtherComp :type "PrimitiveComponent Object Reference") (OtherBodyIndex :type Integer) (bFromSweep :type Boolean) (SweepResult :type "HitResult Structure (by ref)"))
  (`KismetSystemLibrary.Delay` (`self.TimeToDestroy`))
  (cast `/Game/Game/Blueprints/Characters/BP_MyCat` OtherActor)
  (`SceneComponent.SetHiddenInGame` (`self.PaperSprite`) true true)
  (`PrimitiveComponent.SetCollisionEnabled` (`self.Box`) "NoCollision")
  (`PrimitiveComponent.SetCollisionEnabled` (`self.PaperSprite`) "NoCollision")
  (`KismetSystemLibrary.Delay` (`self.TimeToRespawn`))
  (`SceneComponent.SetHiddenInGame` (`self.PaperSprite`) false true)
  (`PrimitiveComponent.SetCollisionEnabled` (`self.Box`) "QueryAndPhysics")
  (`PrimitiveComponent.SetCollisionEnabled` (`self.PaperSprite`) "QueryAndPhysics"))

(fn `UserConstructionScript`
  (`parent.UserConstructionScript`))