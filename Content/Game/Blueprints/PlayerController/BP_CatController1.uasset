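; Player controller for a two-cat game, moving the possessed BP_MyCat and handling pause through the BP_LevelGameMode widget.
; On BeginPlay it spawns a BP_CatController2 to possess the other cat.
; Move input drives this cat's facing, movement and animation, and is forwarded negated so the second cat gets mirrored input, while jumps are relayed as-is.
; Swap exchanges the two cats' world locations rather than changing possession.
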(event `InputAction|Pause`
  (params (Key :type "Key Structure"))
  (:`Pressed`
    (bind _asbp_level_game_mode (cast `/Game/Game/Blueprints/GameModes/BP_LevelGameMode` (`GameplayStatics.GetGameMode`)))
    (bind _pausewidget (`/Game/Game/Blueprints/GameModes/BP_LevelGameMode.PauseWidget` _asbp_level_game_mode))
    (`Widget.SetVisibility` _pausewidget "Visible")
    (set `self.bShowMouseCursor` true)
    (`WidgetBlueprintLibrary.SetInputMode_UIOnlyEx` self _pausewidget)
    (`self.GamePause`)
    (`self.DisableInput` (`GameplayStatics.GetPlayerPawn` 0) self)
    (`GameplayStatics.SetGamePaused` true)))

(event `self.ReceiveBeginPlay`
  (bind _returnvalue (`|SpawnActorFromClass` "/Game/Game/Blueprints/PlayerController/BP_CatController2.BP_CatController2_C" (`KismetMathLibrary.MakeTransform` (0.0 0.0 0.0)) "Undefined" "OverrideRootScale" null null))
  (set `self.AnotherCatController` _returnvalue)
  (bind _outactors (`GameplayStatics.GetAllActorsOfClass` "/Game/Game/Blueprints/Characters/BP_MyCat.BP_MyCat_C"))
  (for _array_element _outactors
    (if (!= _array_element (`self.Cat`))
      (bind _output_get (set `self.AnotherCat` _array_element))
      (`self.Possess` (`self.AnotherCatController`) _output_get)
      (break))))

(event `self.ReceivePossess`
  (params (PossessedPawn :type "Pawn Object Reference"))
  (bind _asbp_my_cat (cast `/Game/Game/Blueprints/Characters/BP_MyCat` PossessedPawn))
  (set `self.Cat` _asbp_my_cat))

(event `InputAxis|MoveRight`
  (params (AxisValue :type "Float (single-precision)"))
  (bind _cat (`self.Cat`))
  (bind _cat_2 (`self.Cat`))
  (bind _cat_3 (`self.Cat`))
  (`/Engine/EditorBlueprintResources/StandardMacros.CompareFloat` AxisValue
    (:`>`
      (set `/Game/Game/Blueprints/Characters/BP_MyCat.IsMoving` true (`self.Cat`))
      (`self.SetControlRotation` (`KismetMathLibrary.MakeRotator` 0.0))
      (`Pawn.AddMovementInput` _cat_3 (1.0 0.0 0.0) (`/Game/Game/Blueprints/Characters/BP_MyCat.Speed Scale` _cat_3) false)
      (`/Game/Game/Blueprints/Characters/BP_MyCat.UpdateAnimation` (`self.Cat`))
      (`/Game/Game/Blueprints/PlayerController/BP_CatController2.MoveRight` (`self.AnotherCatController`) (* AxisValue -1.0) :!label _label))
    (:`==`
      (set `/Game/Game/Blueprints/Characters/BP_MyCat.IsMoving` false (`self.Cat`))
      (`/Game/Game/Blueprints/Characters/BP_MyCat.UpdateAnimation` (`self.Cat`))
      (goto _label))
    (:`<`
      (set `/Game/Game/Blueprints/Characters/BP_MyCat.IsMoving` true _cat)
      (if (not (`/Game/Game/Blueprints/Characters/BP_MyCat.IsHitting` _cat))
        (`self.SetControlRotation` (`KismetMathLibrary.MakeRotator` 0.0 0.0 180.0))
        (`Pawn.AddMovementInput` _cat_2 (-1.0 0.0 0.0) (`/Game/Game/Blueprints/Characters/BP_MyCat.Speed Scale` _cat_2) false)
        (`/Game/Game/Blueprints/Characters/BP_MyCat.UpdateAnimation` (`self.Cat`))
        (goto _label)))))

(event `InputAction|Jump`
  (params (Key :type "Key Structure"))
  (bind _cat (`self.Cat`))
  (:`Pressed`
    (switch `/Game/Game/Blueprints/Data/JumpStates` (`/Game/Game/Blueprints/Characters/BP_MyCat.JumpingState` (`self.Cat`))
      (:`NewEnumerator0`
        (if (not (`/Game/Game/Blueprints/Characters/BP_MyCat.IsHitting` _cat))
          (set `/Game/Game/Blueprints/Characters/BP_MyCat.JumpingState` "NewEnumerator1" _cat)
          (`Character.Jump` (`self.Cat`))
          (`/Game/Game/Blueprints/PlayerController/BP_CatController2.JumpPressed` (`self.AnotherCatController`))
          (`GameplayStatics.PlaySound2D` "/Game/Game/Resources/Sounds/Jump_Cue.Jump_Cue" 1.0 1.0 0.0 null null)))))
  (:`Released`
    (`Character.StopJumping` (`self.Cat`))
    (`/Game/Game/Blueprints/PlayerController/BP_CatController2.JumpReleased` (`self.AnotherCatController`))))

(event `InputAction|Swap`
  (params (Key :type "Key Structure"))
  (:`Pressed`
    (`self.SwapPlayers`)
    (`GameplayStatics.PlaySound2D` "/Game/Game/Resources/Sounds/Swap.Swap" 1.0 1.0 0.0 null null)))

(fn `SwapPlayers`
  (locals (TempLocation :type "Vector Structure"))
  (bind _cat (`self.Cat`))
  (set `local.TempLocation` (`self.K2_GetActorLocation` _cat))
  (`self.K2_SetActorLocation` _cat (`self.K2_GetActorLocation` (`self.AnotherCat`)) false false)
  (`self.K2_SetActorLocation` (`self.AnotherCat`) (`local.TempLocation`) false false))

(fn `UserConstructionScript`)