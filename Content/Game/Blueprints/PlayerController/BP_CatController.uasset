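; Player controller that drives the BP_MyCat character along the X axis and handles pausing.
; On possess it caches the cat, then MoveRight input flips control rotation to face the travel direction, adds movement and updates animation.
; Movement and jump starts are blocked while the cat is hitting, and jumping also requires the Not Jumping state.
; Pause shows the level game mode's pause widget, switches to UI-only input and pauses the game.
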(event `InputAction|Pause`
  (params (Key :type "Key Structure"))
  (:`Pressed`
    (bind _asbp_level_game_mode (cast `/Game/Game/Blueprints/GameModes/BP_LevelGameMode` (`GameplayStatics.GetGameMode`)))
    (bind _pausewidget (`/Game/Game/Blueprints/GameModes/BP_LevelGameMode.PauseWidget` _asbp_level_game_mode))
    (`Widget.SetVisibility` _pausewidget "Visible")
    (set `self.bShowMouseCursor` true)
    (`WidgetBlueprintLibrary.SetInputMode_UIOnlyEx` self _pausewidget)
    (`self.GamePause`)
    (`self.DisableInput` (`GameplayStatics.GetPlayerPawn` 0) self)
    (`GameplayStatics.SetGamePaused` true)))

(event `self.ReceiveBeginPlay`)

(event `self.ReceivePossess`
  (params (PossessedPawn :type "Pawn Object Reference"))
  (bind _asbp_my_cat (cast `/Game/Game/Blueprints/Characters/BP_MyCat` PossessedPawn))
  (set `self.Cat` _asbp_my_cat))

(event `InputAxis|MoveRight`
  (params (AxisValue :type "Float (single-precision)"))
  (bind _cat (`self.Cat`))
  (bind _cat_2 (`self.Cat`))
  (bind _cat_3 (`self.Cat`))
  (bind _cat_4 (`self.Cat`))
  (`/Engine/EditorBlueprintResources/StandardMacros.CompareFloat` AxisValue
    (:`>`
      (set `/Game/Game/Blueprints/Characters/BP_MyCat.IsMoving` true _cat_2)
      (if (not (`/Game/Game/Blueprints/Characters/BP_MyCat.IsHitting` _cat_2))
        (`self.SetControlRotation` (`KismetMathLibrary.MakeRotator` 0.0))
        (`Pawn.AddMovementInput` _cat_4 (1.0 0.0 0.0) (`/Game/Game/Blueprints/Characters/BP_MyCat.Speed Scale` _cat_4) false)
        (`/Game/Game/Blueprints/Characters/BP_MyCat.UpdateAnimation` (`self.Cat`))))
    (:`==`
      (set `/Game/Game/Blueprints/Characters/BP_MyCat.IsMoving` false (`self.Cat`))
      (`/Game/Game/Blueprints/Characters/BP_MyCat.UpdateAnimation` (`self.Cat`)))
    (:`<`
      (set `/Game/Game/Blueprints/Characters/BP_MyCat.IsMoving` true _cat)
      (if (not (`/Game/Game/Blueprints/Characters/BP_MyCat.IsHitting` _cat))
        (`self.SetControlRotation` (`KismetMathLibrary.MakeRotator` 0.0 0.0 180.0))
        (`Pawn.AddMovementInput` _cat_3 (-1.0 0.0 0.0) (`/Game/Game/Blueprints/Characters/BP_MyCat.Speed Scale` _cat_3) false)
        (`/Game/Game/Blueprints/Characters/BP_MyCat.UpdateAnimation` (`self.Cat`))))))

(event `InputAction|Jump`
  (params (Key :type "Key Structure"))
  (bind _cat (`self.Cat`))
  (:`Pressed`
    (switch `/Game/Game/Blueprints/Data/JumpStates` (`/Game/Game/Blueprints/Characters/BP_MyCat.JumpingState` (`self.Cat`))
      (:`NewEnumerator0`
        (if (not (`/Game/Game/Blueprints/Characters/BP_MyCat.IsHitting` _cat))
          (set `/Game/Game/Blueprints/Characters/BP_MyCat.JumpingState` "NewEnumerator1" _cat)
          (`Character.Jump` (`self.Cat`))))))
  (:`Released`
    (`Character.StopJumping` (`self.Cat`))))

(fn `UserConstructionScript`)