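; Player controller for the cat character, handling left/right movement along the world X axis and jumping.
; On possession it caches the BP_AliveCat pawn, then drives it from the MoveRight axis by setting movement state, facing rotation, scaled movement input and animation updates.
; Jumping starts only from the Not Jumping state while not hitting, and release stops it.
; Hitting also blocks leftward movement, but not rightward.
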(event `self.ReceivePossess`
  (params (PossessedPawn :type "Pawn Object Reference"))
  (bind _asbp_alive_cat (cast `/Game/Game/Blueprints/Characters/BP_AliveCat` PossessedPawn))
  (set `self.Cat` _asbp_alive_cat))

(event `MoveRight`
  (params (AxisValue :type "Float (double-precision)"))
  (bind _cat (`self.Cat`))
  (bind _cat_2 (`self.Cat`))
  (bind _cat_3 (`self.Cat`))
  (`/Engine/EditorBlueprintResources/StandardMacros.CompareFloat` AxisValue
    (:`>`
      (set `/Game/Game/Blueprints/Characters/BP_AliveCat.IsMoving` true (`self.Cat`))
      (`self.K2_SetActorRotation` :`self` (`self.Cat`))
      (`Pawn.AddMovementInput` _cat_3 (1.0 0.0 0.0) (`/Game/Game/Blueprints/Characters/BP_AliveCat.Speed Scale` _cat_3) false)
      (`/Game/Game/Blueprints/Characters/BP_AliveCat.UpdateAnimation` (`self.Cat`)))
    (:`==`
      (set `/Game/Game/Blueprints/Characters/BP_AliveCat.IsMoving` false (`self.Cat`))
      (`/Game/Game/Blueprints/Characters/BP_AliveCat.UpdateAnimation` (`self.Cat`)))
    (:`<`
      (set `/Game/Game/Blueprints/Characters/BP_AliveCat.IsMoving` true _cat)
      (if (not (`/Game/Game/Blueprints/Characters/BP_AliveCat.IsHitting` _cat))
        (`self.K2_SetActorRotation` (`self.Cat`) (struct :`Yaw` 180.0) false)
        (`Pawn.AddMovementInput` _cat_2 (-1.0 0.0 0.0) (`/Game/Game/Blueprints/Characters/BP_AliveCat.Speed Scale` _cat_2) false)
        (`/Game/Game/Blueprints/Characters/BP_AliveCat.UpdateAnimation` (`self.Cat`))))))

(event `JumpPressed`
  (bind _cat (`self.Cat`))
  (switch `/Game/Game/Blueprints/Data/JumpStates` (`/Game/Game/Blueprints/Characters/BP_AliveCat.JumpingState` (`self.Cat`))
    (:`NewEnumerator0`
      (if (not (`/Game/Game/Blueprints/Characters/BP_AliveCat.IsHitting` _cat))
        (set `/Game/Game/Blueprints/Characters/BP_AliveCat.JumpingState` "NewEnumerator1" _cat)
        (`Character.Jump` (`self.Cat`))))))

(event `JumpReleased`
  (`Character.StopJumping` (`self.Cat`)))

(fn `UserConstructionScript`)