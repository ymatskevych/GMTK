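; Player controller for the crawl-text game mode that handles the Pause input.
; On press, it shows the PauseWidget held by BP_CrawlTExtGM, enables the cursor and switches to UI-only input focused on that widget.
; It then disables the player pawn's input, pauses the game and calls PauseSound on BP_GameInstance.
; It contains no unpause logic.
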(event `InputAction|Pause`
  (params (Key :type "Key Structure"))
  (:`Pressed`
    (bind _asbp_crawl_text_gm (cast `/Game/Game/Blueprints/GameModes/BP_CrawlTExtGM` (`GameplayStatics.GetGameMode`)))
    (bind _pausewidget (`/Game/Game/Blueprints/GameModes/BP_CrawlTExtGM.PauseWidget` _asbp_crawl_text_gm))
    (`Widget.SetVisibility` _pausewidget "Visible")
    (set `self.bShowMouseCursor` true)
    (`WidgetBlueprintLibrary.SetInputMode_UIOnlyEx` self _pausewidget)
    (`self.DisableInput` (`GameplayStatics.GetPlayerPawn` 0) self)
    (`GameplayStatics.SetGamePaused` true)
    (bind _asbp_game_instance (cast `/Game/Game/Blueprints/GameModes/BP_GameInstance` (`GameplayStatics.GetGameInstance`)))
    (`/Game/Game/Blueprints/GameModes/BP_GameInstance.PauseSound` _asbp_game_instance)))

(fn `UserConstructionScript`)